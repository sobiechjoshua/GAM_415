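; BP_ColoredProjectile is a projectile Blueprint meant to give its mesh a randomized color when play begins.
; BeginPlay creates a dynamic instance of M_Projectile, then multiplies RandomColor from the material parameter collection by a random RGBA color.
; The result is written to parameter "None", although a ParameterName variable is set to "Color".
; A debug print shows a random color generated separately from the applied one.
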(event EventBeginPlay
  (bind _returnvalue (Math|Random|RandomFloatinRange 0.0 1.0))
  (bind _returnvalue_2 (Math|Random|RandomFloatinRange 0.0 1.0))
  (bind _returnvalue_3 (Math|Random|RandomFloatinRange 0.0 1.0))
  (bind _returnvalue_4 (Math|Random|RandomFloatinRange 0.0 1.0))
  (bind _returnvalue_5 (Math|Color|MakeColor _returnvalue_2 _returnvalue_3 _returnvalue_4 _returnvalue))
  (Variables|Default|SetParameter%20Name "Color")
  (bind _returnvalue_6 (Rendering|Material|GetVectorParameterValue "/Game/materials/M_ParamterCollection.M_ParamterCollection" "RandomColor" :!class /Script/Engine.KismetMaterialLibrary))
  (bind _returnvalue_7 (Rendering|Material|CreateDynamicMaterialInstance (Variables|Default|GetProjectileMesh) 0 "/Game/materials/M_Projectile.M_Projectile" "None" :!class /Script/Engine.PrimitiveComponent))
  (Development|PrintString (Utilities|String|ToString(Integer) _returnvalue_5))
  (Rendering|Material|SetVectorParameterValue _returnvalue_7 "" (* _returnvalue_6 _returnvalue_5) :!class /Script/Engine.MaterialInstanceDynamic))

(fn ConstructionScript)